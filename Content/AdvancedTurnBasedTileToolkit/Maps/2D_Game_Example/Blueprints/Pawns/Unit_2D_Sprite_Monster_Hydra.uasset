(event `self.Receive Damage`
  (params (Damage :type "Float (single-precision)") (`Anim Delay` :type "Float (single-precision)"))
  (bind _3_heads (`self.3 Heads`))
  (bind _2_heads (`self.2 Heads`))
  (bind _4_heads (`self.4 Heads`))
  (`parent.Receive Damage` Damage `Anim Delay`)
  (switch `int` (`self.Heads`)
    (:`1`
      (`self.Add Head` (`self.PaperSprite`) _2_heads))
    (:`2`
      (`self.Add Head` _2_heads _3_heads))
    (:`3`
      (`self.Add Head` _3_heads _4_heads))
    (:`4`
      (`self.Add Head` _4_heads (`self.5 Heads`)))))

(event `self.Attack Victim`
  (params (Victim :type "/Game/AdvancedTurnBasedTileToolkit/Blueprints/Pawns/Unit_Parent Object Reference"))
  (bind (_returnvalue_roll _returnvalue_pitch _returnvalue_yaw) (`KismetMathLibrary.BreakRotator` (`self.K2_GetActorRotation`)))
  (bind _gridmanager_ref (`self.GridManager_Ref`))
  (bind _gamemode_ref (`self.GameMode_Ref`))
  (bind (_returnvalue_roll_2 _returnvalue_pitch_2 _returnvalue_yaw_2) (`KismetMathLibrary.BreakRotator` (`KismetMathLibrary.FindLookAtRotation` (`self.AttackerLocation`) (`self.TargetLocation`))))
  (bind _targetmarker (`/Game/AdvancedTurnBasedTileToolkit/Blueprints/Gameplay/BP_Grid_Manager.TargetMarker` _gridmanager_ref))
  (bind _target_marker_decal (`/Game/AdvancedTurnBasedTileToolkit/Blueprints/Gameplay/BP_Grid_Manager.Target Marker Decal` _gridmanager_ref))
  ;[0 0 0] Attack Victim
  (`/Game/AdvancedTurnBasedTileToolkit/Blueprints/Gameplay/BP_Grid_Manager.Set Marker Location` (`self.GridManager_Ref`) (0.0 0.0 0.0) false (`/Game/AdvancedTurnBasedTileToolkit/Blueprints/Pawns/Unit_Parent.Index` Victim) _target_marker_decal _targetmarker)
  (`/Game/AdvancedTurnBasedTileToolkit/Blueprints/Gameplay/BP_Grid_Manager.Set Marker Visibility` (`self.GridManager_Ref`) true _target_marker_decal _targetmarker)
  (set `self.AttackerLocation` (`self.K2_GetActorLocation`))
  (bind _output_get (set `self.TargetLocation` (`self.K2_GetActorLocation` Victim)))
  (`/Engine/EditorBlueprintResources/StandardMacros.IncrementInt` (`self.Attack Count`) :!label _label
    (:`  `
      (if (`self.Projectile`)
        (bind _returnvalue (`|SpawnActorFromClass` (`self.Projectile Class`) (`KismetMathLibrary.Conv_VectorToTransform` (`self.AttackerLocation`)) "Undefined" "OverrideRootScale"))
        (bind (_direction _attack_timeline) (`Timeline|Timeline_4` :!via `PlayFromStart`)
          (:`Update`
            (`self.K2_SetActorLocationAndRotation` _returnvalue (+ (`self.AttackerLocation`) (* (- (`self.TargetLocation`) (`self.AttackerLocation`)) _attack_timeline)) (`KismetMathLibrary.MakeRotator` 0.0 0.0 (+ _returnvalue_yaw_2 90.0)) false false))
          (:`Finished`
            (`self.K2_DestroyActor` _returnvalue)
            (`GameplayStatics.PlaySound2D` (`self.Hit Sound`) :!label _label_2)
            (`self.Receive Damage` Victim (`self.Damage`) 0.0)
            (if (== (`self.Heads`) (`self.Attack Count`))
              (set `self.Attack Count` 0)
              (`/Game/AdvancedTurnBasedTileToolkit/Blueprints/Gameplay/ATBTT_GameMode.ChooseNextPawn` _gamemode_ref (`/Game/AdvancedTurnBasedTileToolkit/Blueprints/Gameplay/ATBTT_GameMode.AI Activation Delay` _gamemode_ref))
              (`self.K2_SetActorLocation` (+ (* (- (`self.TargetLocation`) (`self.AttackerLocation`)) (stale _attack_timeline_2)) (`self.AttackerLocation`)) :!label _label_3)
              (else
                (`KismetSystemLibrary.Delay` 0.2)
                (goto _label)))))
        (else
          (bind (_returnvalue_roll_3 _returnvalue_pitch_3 _returnvalue_yaw_3) (`KismetMathLibrary.BreakRotator` (`KismetMathLibrary.FindLookAtRotation` (`self.K2_GetActorLocation`) _output_get)))
          (if (== (`KismetMathLibrary.Abs` _returnvalue_yaw_3) 90.0)
            (bind (_direction_2 _attack_timeline_2) (`Timeline|Timeline_3` :!via `PlayFromStart` :!label _label_4)
              (:`Update`
                (goto _label_3))
              (:`Attack Hit`
                (goto _label_2)))
            (else
              (`SceneComponent.K2_SetWorldRotation` (`self.Sprite Anchor`) (`KismetMathLibrary.MakeRotator` _returnvalue_roll (* (`KismetMathLibrary.FFloor` (/ (- _returnvalue_yaw_3 90.0) 180.0)) 180.0) _returnvalue_yaw) false false)
              (goto _label_4 :!via `PlayFromStart`))))))))

(event `self.Destroy Unit`
  (params (`Anim Delay` :type "Float (single-precision)"))
  (`parent.Destroy Unit` `Anim Delay`)
  (bind _foundwidgets (`WidgetBlueprintLibrary.GetAllWidgetsOfClass` "/Game/AdvancedTurnBasedTileToolkit/Blueprints/Gameplay/HUD_Faction_Turn.HUD_Faction_Turn_C"))
  (bind _ashud_faction_turn (cast `/Game/AdvancedTurnBasedTileToolkit/Blueprints/Gameplay/HUD_Faction_Turn` (`KismetArrayLibrary.Array_Get` _foundwidgets))
    (:`then`
      (`TextBlock.SetText` (`/Game/AdvancedTurnBasedTileToolkit/Blueprints/Gameplay/HUD_Faction_Turn.text_game_over` _ashud_faction_turn) "YOU WIN!")
      (`/Game/AdvancedTurnBasedTileToolkit/Blueprints/Gameplay/HUD_Faction_Turn.Game Over HUD` _ashud_faction_turn))
    (:`CastFailed`
      _))
  (set `/Game/AdvancedTurnBasedTileToolkit/Blueprints/Gameplay/ATBTT_GameMode.Game Over` true (`self.GameMode_Ref`)))

(fn `Add Head`
  (params (`Old Sprite` :type "SceneComponent Object Reference") (`New Sprite` :type "SceneComponent Object Reference"))
  (`SceneComponent.SetVisibility` `Old Sprite` false false)
  (`SceneComponent.SetVisibility` `New Sprite` true false)
  (`/Engine/EditorBlueprintResources/StandardMacros.IncrementInt` (`self.Heads`)
    (:`  `
      (return))))

(fn `UserConstructionScript`
  (`parent.UserConstructionScript`))
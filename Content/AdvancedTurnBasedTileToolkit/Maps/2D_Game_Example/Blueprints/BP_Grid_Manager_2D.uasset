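; Grid manager for the 2D dungeon example, adding fog of war and free-roam exploration to the turn-based tile toolkit.
; Activation creates the HUD, covers tiles with instanced fog planes and starts free roam with only the hero in initiative.
; RevealVisibleTiles line-traces to tiles in range, clearing visible fog, adding discovered pawns to initiative and halting the hero to end free roam.
; The overridden pathfinding search admits only revealed tiles.
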(event `self.Activate Grid Manager`
  ;[1 1 1] On Activation
  (`parent.Activate Grid Manager`)
  (bind _returnvalue (`|CreateWidget` "/Game/AdvancedTurnBasedTileToolkit/Maps/2D_Game_Example/Blueprints/DungeonHUD.DungeonHUD_C"))
  (`UserWidget.AddToViewport` _returnvalue 0)
  (bind _returnvalue_2 (`AddComponent|InstancedStaticMeshComponent_0`))
  (bind _output_get (set `self.Fog of War Instance` _returnvalue_2))
  (`StaticMeshComponent.SetStaticMesh` _output_get "/Game/AdvancedTurnBasedTileToolkit/Meshes/simple_plane_UV.simple_plane_UV")
  (for _array_element (`self.VectorFieldArray`)
    (`InstancedStaticMeshComponent.AddInstance` (`self.Fog of War Instance`) (`KismetMathLibrary.MakeTransform` (`KismetMathLibrary.MakeVector` (.x _array_element) (.y _array_element) (+ (.z _array_element) 1.0)))))
  (`KismetArrayLibrary.Array_Resize` (`self.Fog of War Array`) (* (`self.GridSizeX`) (`self.GridSizeY`))) ; Fills the array keeping tracks of which tiles have been revealed
  (bind _asatbtt_game_mode (cast `/Game/AdvancedTurnBasedTileToolkit/Blueprints/Gameplay/ATBTT_GameMode` (`GameplayStatics.GetGameMode`))) ; Clears the Initiative order and then adds only the hero
  (bind _initiativeorder (`/Game/AdvancedTurnBasedTileToolkit/Blueprints/Gameplay/ATBTT_GameMode.InitiativeOrder` _asatbtt_game_mode))
  (`KismetArrayLibrary.Array_Clear` _initiativeorder)
  (bind _outactors (`GameplayStatics.GetAllActorsOfClass` (`self.Hero Ref`)))
  (`KismetArrayLibrary.Array_Add` _initiativeorder (`KismetArrayLibrary.Array_Get` _outactors))
  (set `/Game/AdvancedTurnBasedTileToolkit/Blueprints/Gameplay/ATBTT_GameMode.FreeRoam` true _asatbtt_game_mode)
  (bind _foundwidgets (`WidgetBlueprintLibrary.GetAllWidgetsOfClass` "/Game/AdvancedTurnBasedTileToolkit/Blueprints/Gameplay/HUD_Faction_Turn.HUD_Faction_Turn_C"))
  (`Widget.SetVisibility` (`/Game/AdvancedTurnBasedTileToolkit/Blueprints/Gameplay/HUD_Faction_Turn.TurnText` (`KismetArrayLibrary.Array_Get` _foundwidgets)) "Hidden"))

(event `self.Search and add adjacent tiles (Custom 1)`
  (for _array_element (`self.OpenList`)
    (if (== (`self.CurrentSearchStep`) (`.Cost_6_814E1E3C4BD931C65DCA6E85ABE78039` (break `/Game/AdvancedTurnBasedTileToolkit/Blueprints/Gameplay/Structs/Struct_Pathfinding` _array_element)))
      (bind _item_edge_array_tile (break `/Game/AdvancedTurnBasedTileToolkit/Blueprints/Gameplay/Structs/Struct_Edge_Array_Tile` (`KismetArrayLibrary.Array_Get` (`self.Edge Array`) (break `/Game/AdvancedTurnBasedTileToolkit/Blueprints/Gameplay/Structs/Struct_Pathfinding` _array_element))))
      (for _array_element_2 _item_edge_array_tile
        (bind (_item_index _item_cost) (break `/Game/AdvancedTurnBasedTileToolkit/Blueprints/Gameplay/Structs/Struct_Pathfinding` (`KismetArrayLibrary.Array_Get` (`self.CanMoveToArray`) (break `/Game/AdvancedTurnBasedTileToolkit/Blueprints/Gameplay/Structs/Struct_Index_Cost` _array_element_2))))
        ;[0.015 0.015 0.015] Looks at the node in the specified location relative to a "parent" node. Adds the node to the open list (becoming a new parent later) if the following  conditions are met:
        (if (== _item_cost 0)
          ;;[0 0.1668 1] Nodes specific to this blueprint.
          ;; Makes it so that the player cannot
          ;; enter tiles that are not yet visible.
          (if (`KismetArrayLibrary.Array_Get` (`self.Fog of War Array`) (break `/Game/AdvancedTurnBasedTileToolkit/Blueprints/Gameplay/Structs/Struct_Index_Cost` _array_element_2))
            (if (!= (`KismetArrayLibrary.Array_Get` (`self.Pawn Array`) (break `/Game/AdvancedTurnBasedTileToolkit/Blueprints/Gameplay/Structs/Struct_Index_Cost` _array_element_2)) null)
              (`KismetArrayLibrary.Array_Add` (`self.Reachable_Pawns_Array`) (break `/Game/AdvancedTurnBasedTileToolkit/Blueprints/Gameplay/Structs/Struct_Index_Cost` _array_element_2)) ; For AI: Add any reachable player pawns to the reachable pawns array for later choosing a target
              (bind _returnvalue (+ (`.Cost_5_A9F9F0E74CF53F1494DAC5BEA2D7E35B` (break `/Game/AdvancedTurnBasedTileToolkit/Blueprints/Gameplay/Structs/Struct_Index_Cost` _array_element_2)) (`.Cost_6_814E1E3C4BD931C65DCA6E85ABE78039` (break `/Game/AdvancedTurnBasedTileToolkit/Blueprints/Gameplay/Structs/Struct_Pathfinding` _array_element))))
              (`KismetArrayLibrary.Array_Set` (`self.CanMoveToArray`) (break `/Game/AdvancedTurnBasedTileToolkit/Blueprints/Gameplay/Structs/Struct_Index_Cost` _array_element_2) (make `/Game/AdvancedTurnBasedTileToolkit/Blueprints/Gameplay/Structs/Struct_Pathfinding` 0 _returnvalue (break `/Game/AdvancedTurnBasedTileToolkit/Blueprints/Gameplay/Structs/Struct_Pathfinding` _array_element)) :!label _label) ; The can move to array stores all nodes a pawn can move to
              (elif (<= _returnvalue (`self.Max Move`))
                (`KismetArrayLibrary.Array_Add` (`self.OpenListChildren`) (make `/Game/AdvancedTurnBasedTileToolkit/Blueprints/Gameplay/Structs/Struct_Pathfinding` (break `/Game/AdvancedTurnBasedTileToolkit/Blueprints/Gameplay/Structs/Struct_Index_Cost` _array_element_2) _returnvalue (break `/Game/AdvancedTurnBasedTileToolkit/Blueprints/Gameplay/Structs/Struct_Pathfinding` _array_element))) ; Add to the open list, becoming a parent itself
                (goto _label)
                (elif (<= (`.Cost_5_A9F9F0E74CF53F1494DAC5BEA2D7E35B` (break `/Game/AdvancedTurnBasedTileToolkit/Blueprints/Gameplay/Structs/Struct_Index_Cost` _array_element_2)) (`self.Max Move`))
                  (`KismetArrayLibrary.Array_Add` (`self.DelayedSearchList`) (make `/Game/AdvancedTurnBasedTileToolkit/Blueprints/Gameplay/Structs/Struct_Pathfinding` (break `/Game/AdvancedTurnBasedTileToolkit/Blueprints/Gameplay/Structs/Struct_Index_Cost` _array_element_2) _returnvalue (break `/Game/AdvancedTurnBasedTileToolkit/Blueprints/Gameplay/Structs/Struct_Pathfinding` _array_element)))))))))
      (else
        (`KismetArrayLibrary.Array_Add` (`self.DelayedSearchList`) (make `/Game/AdvancedTurnBasedTileToolkit/Blueprints/Gameplay/Structs/Struct_Pathfinding` (break `/Game/AdvancedTurnBasedTileToolkit/Blueprints/Gameplay/Structs/Struct_Pathfinding` _array_element) (`.Cost_6_814E1E3C4BD931C65DCA6E85ABE78039` (break `/Game/AdvancedTurnBasedTileToolkit/Blueprints/Gameplay/Structs/Struct_Pathfinding` _array_element)) (`.Parent_9_0C00A7F84152DF85DBC6BABA34152BFA` (break `/Game/AdvancedTurnBasedTileToolkit/Blueprints/Gameplay/Structs/Struct_Pathfinding` _array_element))))))))

(event `self.Reset pathfinding arrays and clear meshes`
  ;[1 1 1] Reset Pathfinding Arrays and Clear Meshes Override
  (`parent.Reset pathfinding arrays and clear meshes`)
  (bind _asatbtt_game_mode (cast `/Game/AdvancedTurnBasedTileToolkit/Blueprints/Gameplay/ATBTT_GameMode` (`GameplayStatics.GetGameMode`)))
  (set `self.Player Turn` (`/Game/AdvancedTurnBasedTileToolkit/Blueprints/Gameplay/ATBTT_GameMode.PlayerTurn` _asatbtt_game_mode)))

(event `self.Set Marker Location`
  (params (Location :type "Vector Structure") (`Use Index` :type Boolean) (Index :type Integer) (`Decal Component` :type "DecalComponent Object Reference") (`SM Component` :type "StaticMeshComponent Object Reference"))
  ;[1 1 1] Set Marker Location Override
  (if (`self.Use Decals`)
    (`SceneComponent.K2_SetRelativeLocation` `Decal Component` (select `bool` `Use Index` :`false` (- Location (`self.K2_GetActorLocation`)) :`true` (`KismetArrayLibrary.Array_Get` (`self.VectorFieldArray`) Index)) false false)
    (else
      (`SceneComponent.K2_SetWorldLocationAndRotation` `SM Component` (select `bool` `Use Index` :`false` (`KismetMathLibrary.MakeVector` (.x Location) (.y Location) (+ (.z Location) 0.3)) :`true` (`self.Index To Vector on Grid` Index 0.3)) (`KismetArrayLibrary.Array_Get` (`self.RotatorArray`) Index) false false))))

(fn `Reveal Visible Tiles`
  (params (Index :type Integer) (Range :type Integer))
  (locals (`Local Index` :type Integer))
  (bind _returnvalue (`self.K2_GetActorLocation`))
  (bind _visibilitytraceheight (`self.VisibilityTraceHeight`))
  (bind (_item_x _item_y _item_z) (`KismetMathLibrary.BreakVector` (`KismetArrayLibrary.Array_Get` (`self.VectorFieldArray`) (`local.Local Index`))))
  (bind _output_get (set `local.Local Index` Index))
  (`self.Get Indexes in Range` _output_get Range)
  (for _array_element (`self.TilesInRangeArray`)
    (if (not (`KismetArrayLibrary.Array_Get` (`self.Fog of War Array`) (break `/Game/AdvancedTurnBasedTileToolkit/Blueprints/Gameplay/Structs/Struct_Range` _array_element)))
      (bind (_returnvalue_x _returnvalue_y _returnvalue_z) (`KismetMathLibrary.BreakVector` (+ (`KismetArrayLibrary.Array_Get` (`self.VectorFieldArray`) (break `/Game/AdvancedTurnBasedTileToolkit/Blueprints/Gameplay/Structs/Struct_Range` _array_element)) (`self.K2_GetActorLocation`))))
      (bind (_outhit _returnvalue_2) (`KismetSystemLibrary.LineTraceSingle` (`KismetMathLibrary.MakeVector` _item_x _item_y (+ _item_z _visibilitytraceheight)) (`KismetMathLibrary.MakeVector` _returnvalue_x _returnvalue_y (+ _visibilitytraceheight _returnvalue_z)) "TraceTypeQuery4"))
      (if _returnvalue_2
        (bind _item (`KismetArrayLibrary.Array_Get` (`self.VectorFieldArray`) (break `/Game/AdvancedTurnBasedTileToolkit/Blueprints/Gameplay/Structs/Struct_Range` _array_element)))
        (if (== (`.Location` (`GameplayStatics.BreakHitResult` _outhit)) (+ _item _returnvalue) :`ErrorTolerance` 220.0)
          (bind (_returnvalue_x_2 _returnvalue_y_2 _returnvalue_z_2) (`KismetMathLibrary.BreakVector` (+ _item _returnvalue)))
          (bind _item_2 (`KismetArrayLibrary.Array_Get` (`InstancedStaticMeshComponent.GetInstancesOverlappingSphere` (`self.Fog of War Instance`) (`KismetMathLibrary.MakeVector` _returnvalue_x_2 _returnvalue_y_2 (+ _returnvalue_z_2 20.0)) 20.0 true)))
          (if (!= _item_2 0) :!label _label
            (`InstancedStaticMeshComponent.UpdateInstanceTransform` (`self.Fog of War Instance`) _item_2 (`KismetMathLibrary.MakeTransform` (0.0 0.0 0.0)) false true false)
            (`KismetArrayLibrary.Array_Set` (`self.Fog of War Array`) (break `/Game/AdvancedTurnBasedTileToolkit/Blueprints/Gameplay/Structs/Struct_Range` _array_element) true)
            (bind _item_3 (`KismetArrayLibrary.Array_Get` (`self.Pawn Array`) (break `/Game/AdvancedTurnBasedTileToolkit/Blueprints/Gameplay/Structs/Struct_Range` _array_element)))
            (if (!= _item_3 null)
              (bind _asatbtt_game_mode (cast `/Game/AdvancedTurnBasedTileToolkit/Blueprints/Gameplay/ATBTT_GameMode` (`GameplayStatics.GetGameMode`)))
              (if (!= (break `/Game/AdvancedTurnBasedTileToolkit/Blueprints/Gameplay/Structs/Struct_Range` _array_element) (`local.Local Index`))
                (`KismetArrayLibrary.Array_AddUnique` (`/Game/AdvancedTurnBasedTileToolkit/Blueprints/Gameplay/ATBTT_GameMode.InitiativeOrder` _asatbtt_game_mode) _item_3)
                (if (`/Game/AdvancedTurnBasedTileToolkit/Blueprints/Gameplay/ATBTT_GameMode.FreeRoam` _asatbtt_game_mode)
                  (bind _asunit_2d_sprite_hero (cast `/Game/AdvancedTurnBasedTileToolkit/Maps/2D_Game_Example/Blueprints/Pawns/Unit_2D_Sprite_Hero` (`/Game/AdvancedTurnBasedTileToolkit/Blueprints/Gameplay/ATBTT_GameMode.CurrentPawn` _asatbtt_game_mode)))
                  (set `/Game/AdvancedTurnBasedTileToolkit/Blueprints/Pawns/Unit_Parent.Stop X tiles from Target` (`/Game/AdvancedTurnBasedTileToolkit/Maps/2D_Game_Example/Blueprints/Pawns/Unit_Parent_2D.TempIntCounter` _asunit_2d_sprite_hero) _asunit_2d_sprite_hero)
                  (set `/Game/AdvancedTurnBasedTileToolkit/Blueprints/Pawns/Unit_Parent.Current Move` 0 _asunit_2d_sprite_hero)
                  (set `/Game/AdvancedTurnBasedTileToolkit/Blueprints/Gameplay/ATBTT_GameMode.FreeRoam` false _asatbtt_game_mode))))))
        (else
          (goto _label))))))

(fn `UserConstructionScript`
  (`parent.UserConstructionScript`))